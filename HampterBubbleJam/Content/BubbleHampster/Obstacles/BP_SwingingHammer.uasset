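; BP_SwingingHammer is an obstacle that swings its Sphere component like a hammer.
; On BeginPlay it waits a random whole number of seconds, under ten, then plays a timeline, so instances can swing out of phase.
; The timeline's HammerSwinging track sets the Sphere's relative rotation each update, with the RotationSwitch flag choosing pitch or roll as the swing axis.
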(event `self.ReceiveBeginPlay`
  (bind _sphere (`self.Sphere`))
  (`KismetSystemLibrary.Delay` (`KismetMathLibrary.Conv_IntToDouble` (`KismetMathLibrary.RandomInteger` 10)))
  (bind (_direction _hammerswinging) (`Timeline|Timeline`)
    (:`Update`
      (if (`self.RotationSwitch`)
        (`SceneComponent.K2_SetRelativeRotation` _sphere (`KismetMathLibrary.MakeRotator` 0.0 _hammerswinging) false false)
        (else
          (`SceneComponent.K2_SetRelativeRotation` _sphere (`KismetMathLibrary.MakeRotator` _hammerswinging) false false))))))

(fn `UserConstructionScript`)