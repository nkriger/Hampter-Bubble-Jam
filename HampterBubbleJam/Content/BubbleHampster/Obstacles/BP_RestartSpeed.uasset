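; BP_RestartSpeed is an obstacle zone that changes how the hamster ball rolls while it overlaps, apparently to slow it down.
; On begin overlap with a BP_HamsterController, it caches the sphere collision's angular damping and replaces it with SlowForce.
; On end overlap it restores the cached value, which is held in a single variable on the zone.
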(event `self.ReceiveActorBeginOverlap`
  (params (OtherActor :type "Actor Object Reference"))
  (bind _asbp_hamster_controller (cast `/Game/BubbleHampster/PlayerHampster/BP_HamsterController` OtherActor))
  (bind _spherecollision (`/Game/BubbleHampster/PlayerHampster/BP_HamsterController.SphereCollision` _asbp_hamster_controller))
  (set `self.CurrentAngDamp` (`PrimitiveComponent.GetAngularDamping` _spherecollision))
  (`PrimitiveComponent.SetAngularDamping` _spherecollision (`self.SlowForce`)))

(event `self.ReceiveActorEndOverlap`
  (params (OtherActor :type "Actor Object Reference"))
  (bind _asbp_hamster_controller (cast `/Game/BubbleHampster/PlayerHampster/BP_HamsterController` OtherActor))
  (`PrimitiveComponent.SetAngularDamping` (`/Game/BubbleHampster/PlayerHampster/BP_HamsterController.SphereCollision` _asbp_hamster_controller) (`self.CurrentAngDamp`)))

(fn `UserConstructionScript`)