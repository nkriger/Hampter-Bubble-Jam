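; BP_WallBounce is an obstacle that launches the hamster along the direction of its Arrow component when touched.
; It stores the Arrow's forward vector in a boost pad stats struct at BeginPlay and refreshes it on each overlap.
; When the overlapping actor is a BP_HamsterController, it applies an impulse of that direction times the boost strength to the hamster's collision sphere.
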(event `self.ReceiveBeginPlay`
  (bind _structout (setmembers `/Game/BubbleHampster/Obstacles/BoostPad/S_BoostPadData` :`StructRef` (`self.BoostStats`) :`Boost Direciton` (`SceneComponent.GetForwardVector` (`self.Arrow`))))
  (set `self.BoostStats` _structout))

(event `self.ReceiveActorBeginOverlap`
  (params (OtherActor :type "Actor Object Reference"))
  (bind (_booststats_booststrngth _booststats_boostdireciton) (break `/Game/BubbleHampster/Obstacles/BoostPad/S_BoostPadData` (`self.BoostStats`)))
  (bind _structout (setmembers `/Game/BubbleHampster/Obstacles/BoostPad/S_BoostPadData` :`StructRef` (`self.BoostStats`) :`Boost Direciton` (`SceneComponent.GetForwardVector` (`self.Arrow`))))
  (set `self.BoostStats` _structout)
  (bind _asbp_hamster_controller (cast `/Game/BubbleHampster/PlayerHampster/BP_HamsterController` OtherActor))
  (`PrimitiveComponent.AddImpulse` (`/Game/BubbleHampster/PlayerHampster/BP_HamsterController.SphereCollision` _asbp_hamster_controller) (* _booststats_boostdireciton _booststats_booststrngth) "None" false))

(fn `UserConstructionScript`)