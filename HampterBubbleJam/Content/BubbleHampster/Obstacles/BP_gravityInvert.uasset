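; BP_gravityInvert is an obstacle volume that works like a fan, pushing hamster players that enter it.
; Overlap adds each BP_HamsterController to a list, and every Tick applies FanForce to its Sphere along the Arrow's forward vector.
; Players no longer overlapping the Box are gathered in a second list and removed after the loop.
; The construction script toggles the Plane's visibility from FanVisible.
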(event `self.ReceiveActorBeginOverlap`
  (params (OtherActor :type "Actor Object Reference"))
  ; Player Enters Zone
  (bind _asbp_hamster_controller (cast `/Game/BubbleHampster/PlayerHampster/BP_HamsterController` OtherActor))
  (`KismetArrayLibrary.Array_Add` (`self.PlayersInFan`) _asbp_hamster_controller))

(event `self.ReceiveTick`
  (params (DeltaSeconds :type "Float (single-precision)"))
  ; Check if at least one player is in fan
  (if (`KismetArrayLibrary.Array_IsNotEmpty` (`self.PlayersInFan`))
    (for _array_element (`self.PlayersInFan`)
      (if (`PrimitiveComponent.IsOverlappingActor` (`self.Box`) _array_element)
        ; Force Add
        (`PrimitiveComponent.AddForce` (`/Game/BubbleHampster/PlayerHampster/BP_HamsterController.Sphere` _array_element) (* (`SceneComponent.GetForwardVector` (`self.Arrow`)) (`self.FanForce`)) "None" false)
        (else
          (`KismetArrayLibrary.Array_Add` (`self.PlayersToRemove`) _array_element))))
    (if (`KismetArrayLibrary.Array_IsNotEmpty` (`self.PlayersToRemove`))
      (for _array_element_2 (`self.PlayersToRemove`)
        (`KismetArrayLibrary.Array_RemoveItem` (`self.PlayersInFan`) _array_element_2)
        (`KismetSystemLibrary.PrintString` "Player Removed"))
      (`KismetArrayLibrary.Array_Clear` (`self.PlayersToRemove`)))))

(fn `UserConstructionScript`
  (`SceneComponent.SetVisibility` (`self.Plane`) (`self.FanVisible`) false))