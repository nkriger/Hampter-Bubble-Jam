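; BP_BubbleVatorSpawner is an obstacle spawner that emits a BP_BubbleVator bubble at its own location when play begins.
; BeginPlay calls SpawnBubbles, which always spawns regardless of collision, schedules the bubble's self-destruct with BubbleLifeSpan and sets its direction from the Arrow component's forward vector.
; The event ends in a SpawnRate delay with nothing shown after it, so no repeat spawn appears in the graph.
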(event `self.ReceiveBeginPlay`
  (`self.SpawnBubbles`))

(event `SpawnBubbles`
  (bind _returnvalue (`|SpawnActorFromClass` "/Game/BubbleHampster/Obstacles/BubbleVator/BP_BubbleVator.BP_BubbleVator_C" (`KismetMathLibrary.MakeTransform` (`self.K2_GetActorLocation`)) "AlwaysSpawn" "MultiplyWithRoot" null null))
  (`/Game/BubbleHampster/Obstacles/BubbleVator/BP_BubbleVator.SelfDestruct` _returnvalue (`self.BubbleLifeSpan`))
  (set `/Game/BubbleHampster/Obstacles/BubbleVator/BP_BubbleVator.BubbleDir` (`SceneComponent.GetForwardVector` (`self.Arrow`)) _returnvalue)
  (`KismetSystemLibrary.Delay` (`self.SpawnRate`)))

(fn `UserConstructionScript`)