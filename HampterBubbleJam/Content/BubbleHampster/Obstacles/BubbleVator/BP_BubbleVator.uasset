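; BP_BubbleVator is a bubble obstacle that captures the hamster and carries it along a spline.
; A spawner supplies the spline and lifespan through GetSpawner, and movement starts one tick after BeginPlay on a rate-scaled timeline.
; Overlap snaps the hamster to the bubble, disables its sphere physics and attaches it, guarded by PlayerInBubble, which is never set here.
; At the spline's end, SelfDestruct restores physics, detaches the hamster and destroys the bubble.
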(event `MoveBubble`
  (`TimelineComponent.SetPlayRate` (`self.MoveTimeline`) (/ 1.0 (`self.TimeToComplete`)))
  (bind (_direction _alpha) (`Timeline|MoveTimeline`)
    (:`Update`
      (`self.K2_SetActorTransform` (`KismetMathLibrary.MakeTransform` (`SplineComponent.GetLocationAtDistanceAlongSpline` (`self.Spline`) (`KismetMathLibrary.Lerp` 0.0 (`SplineComponent.GetSplineLength` (`self.Spline`)) _alpha) "World"))))
    (:`Finished`
      (`self.SelfDestruct`))))

(event `GetSpawner`
  (params (Spawner :type "/Game/BubbleHampster/Obstacles/BubbleVator/BP_BubbleVatorSpawner Object Reference"))
  (bind _output_get (set `self.Spawner` Spawner))
  (set `self.TimeToComplete` (`/Game/BubbleHampster/Obstacles/BubbleVator/BP_BubbleVatorSpawner.BubbleLifeSpan` _output_get))
  (set `self.Spline` (`/Game/BubbleHampster/Obstacles/BubbleVator/BP_BubbleVatorSpawner.Spline` (`self.Spawner`))))

(event `self.ReceiveBeginPlay`
  (`KismetSystemLibrary.DelayUntilNextTick`)
  (`self.MoveBubble`))

(event `self.ReceiveActorBeginOverlap`
  (params (OtherActor :type "Actor Object Reference"))
  (if (not (`self.PlayerInBubble`))
    (bind _asbp_hamster_controller (cast `/Game/BubbleHampster/PlayerHampster/BP_HamsterController` OtherActor))
    (bind _output_get (set `self.Player` _asbp_hamster_controller))
    (`self.K2_SetActorLocation` _output_get (`self.K2_GetActorLocation`) false false)
    (`PrimitiveComponent.SetSimulatePhysics` (`/Game/BubbleHampster/PlayerHampster/BP_HamsterController.SphereCollision` _output_get) false)
    (`self.K2_AttachToActor` _output_get self "None" "KeepWorld" "KeepWorld" "KeepWorld" true)))

(event `self.ReceiveTick`
  (params (DeltaSeconds :type "Float (single-precision)")))

(event `SelfDestruct`
  (`PrimitiveComponent.SetSimulatePhysics` (`/Game/BubbleHampster/PlayerHampster/BP_HamsterController.SphereCollision` (`self.Player`)) true)
  (`self.K2_DetachFromActor` (`self.Player`) "KeepWorld" "KeepWorld" "KeepWorld")
  (`self.K2_DestroyActor`))

(fn `UserConstructionScript`)