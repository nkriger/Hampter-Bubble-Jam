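; BP_HamsterController is the player-controlled hamster, moved as a physics sphere through Enhanced Input.
; BeginPlay loops over all hamster instances, adding the default mapping context to the player controller at each index.
; Look drives control rotation, while Move applies camera-yaw-relative forces to the sphere, stronger forward/back than sideways.
; Jump charges with hold time, prints debug progress, and on completion applies scaled upward force if a downward trace finds ground close below.
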(event `self.ReceiveBeginPlay`
  ;[0.05133 0.15 0.03186 0.5] Player Input Mapping
  (bind _outactors (`GameplayStatics.GetAllActorsOfClass` "BP_HamsterController_C"))
  (for (_ _array_index) _outactors
    (`EnhancedInputSubsystemInterface.AddMappingContext` (pcsubsystem `EnhancedInputLocalPlayerSubsystem` (`GameplayStatics.GetPlayerController` _array_index)) "/Game/ThirdPerson/Input/IMC_Default.IMC_Default" 0 (struct))))

(event `EnhancedInput|/Game/ThirdPerson/Input/Actions/IA_Look`
  (params (ActionValue :type "Vector2D Structure") (ElapsedSeconds :type "Float (double-precision)") (TriggeredSeconds :type "Float (double-precision)") (InputAction :type "InputAction Object Reference" :default "/Game/ThirdPerson/Input/Actions/IA_Look.IA_Look"))
  ;[0.15 0.0872 0.0361 0.5] Looking
  (:`Triggered`
    (`self.AddControllerPitchInput` ActionValue_Y)
    (`self.AddControllerYawInput` ActionValue_X)))

(event `EnhancedInput|/Game/ThirdPerson/Input/Actions/IA_Move`
  (params (ActionValue :type "Vector2D Structure") (ElapsedSeconds :type "Float (double-precision)") (TriggeredSeconds :type "Float (double-precision)") (InputAction :type "InputAction Object Reference" :default "/Game/ThirdPerson/Input/Actions/IA_Move.IA_Move"))
  (bind (_returnvalue_roll _returnvalue_pitch _returnvalue_yaw) (`KismetMathLibrary.BreakRotator` (`self.GetControlRotation`)))
  (bind _spherecollision (`self.SphereCollision`))
  (bind _returnvalue (`KismetMathLibrary.MakeRotator` 0.0 0.0 _returnvalue_yaw))
  ;[0.15 0.05 0.05 0.5] Moving
  (:`Triggered`
    (`PrimitiveComponent.AddForce` _spherecollision (* (`KismetMathLibrary.GetForwardVector` _returnvalue) ActionValue_Y 50000.0) "None" false)
    (`PrimitiveComponent.AddForce` _spherecollision (* (`KismetMathLibrary.GetRightVector` _returnvalue) ActionValue_X 30000.0) "None" false)))

(event `EnhancedInput|/Game/ThirdPerson/Input/Actions/IA_Jump`
  (params (ActionValue :type Boolean) (ElapsedSeconds :type "Float (double-precision)") (TriggeredSeconds :type "Float (double-precision)") (InputAction :type "InputAction Object Reference" :default "/Game/ThirdPerson/Input/Actions/IA_Jump.IA_Jump"))
  (bind _spherecollision (`self.SphereCollision`))
  (bind _returnvalue (`KismetMathLibrary.FClamp` (`KismetMathLibrary.NormalizeToRange` ElapsedSeconds 0.0 1.0) 0.0 1.5))
  (bind _returnvalue_2 (`SceneComponent.K2_GetComponentLocation` _spherecollision))
  (bind _returnvalue_3 (`KismetStringLibrary.Conv_DoubleToString` _returnvalue))
  ;[0.15 0.1457 0.02644 0.5] Jumping
  (:`Started`
    (`KismetSystemLibrary.PrintString` "Started Charging the Jump"))
  (:`Ongoing`
    (`KismetSystemLibrary.PrintString` (`KismetStringLibrary.Concat_StrStr` "Jump Charge: " _returnvalue_3) true true (struct :`R` 0.0625 :`G` 0.169842 :`B` 1.0 :`A` 1.0) 0.0))
  (:`Completed`
    (`KismetSystemLibrary.PrintString` (`KismetStringLibrary.Concat_StrStr` "Charged jump to: " _returnvalue_3))
    (bind _outhit (`KismetSystemLibrary.LineTraceSingle` _returnvalue_2 (- _returnvalue_2 (0.0 0.0 15000.0)) "TraceTypeQuery1"))
    (if (<= (`.Distance` (`GameplayStatics.BreakHitResult` _outhit)) 52.0)
      (`PrimitiveComponent.AddForce` _spherecollision (`KismetMathLibrary.MakeVector` 0.0 0.0 (* _returnvalue 7000000.0)) "None" false))))

(fn `UserConstructionScript`)