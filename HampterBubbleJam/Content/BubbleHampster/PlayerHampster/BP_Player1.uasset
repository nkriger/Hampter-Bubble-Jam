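; Player 1 pawn for BubbleHampster that pulls Player 2 toward itself while the two overlap.
; Beginning an overlap with BP_Player2 stores that player and sets PlayerBehind; any overlap ending clears the flag.
; While the flag is set, Tick runs after the parent's and pushes Player 2's SphereCollision toward this sphere, using ForceStrength scaled by delta time.
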(event `self.ReceiveActorBeginOverlap`
  (params (OtherActor :type "Actor Object Reference"))
  (bind _asbp_player_2 (cast `/Game/BubbleHampster/PlayerHampster/BP_Player2` OtherActor))
  (set `self.Player` _asbp_player_2)
  (set `self.PlayerBehind` true))

(event `self.ReceiveTick`
  (params (DeltaSeconds :type "Float (single-precision)"))
  (bind _spherecollision (`/Game/BubbleHampster/PlayerHampster/BP_HamsterController.SphereCollision` (`self.Player`)))
  (`parent.ReceiveTick` DeltaSeconds)
  (if (`self.PlayerBehind`)
    (`PrimitiveComponent.AddForce` _spherecollision (* (`KismetMathLibrary.GetDirectionUnitVector` (`SceneComponent.K2_GetComponentLocation` _spherecollision) (`SceneComponent.K2_GetComponentLocation` (`self.SphereCollision`))) (`self.ForceStrength`) DeltaSeconds) "None" false)))

(event `self.ReceiveActorEndOverlap`
  (params (OtherActor :type "Actor Object Reference"))
  (set `self.PlayerBehind` false))

(fn `UserConstructionScript`
  (`parent.UserConstructionScript`))